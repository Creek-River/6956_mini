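; BP_rock is a rock actor that destroys itself and damages the player after repeated hits from the eye character.
; Its Hit event identifies that character by comparing display names and increments a counter that is reset on BeginPlay.
; From the second hit, it calls DestroyActor, then applies damage to player character 0.
; A delayed self-destroy chain is left unconnected and never runs.
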(event EventBeginPlay
  (Variables|Default|Setnum 0))

(event Collision|EventActorBeginOverlap
  (params (OtherActor :type Actor%20Object%20Reference)))

(event EventTick
  (params (DeltaSeconds :type Float%20%28single-precision%29)))

(event Collision|EventHit
  (params (MyComp :type Primitive%20Component%20Object%20Reference) (Other :type Actor%20Object%20Reference) (OtherComp :type Primitive%20Component%20Object%20Reference) (bSelfMoved :type Boolean) (HitLocation :type Vector :default "0, 0, 0") (HitNormal :type Vector :default "0, 0, 0") (NormalImpulse :type Vector :default "0, 0, 0") (Hit :type Hit%20Result%20Structure%20%28by%20ref%29))
  (if (Utilities|Enum|Equal(Enum) (Utilities|GetDisplayName Other) (Utilities|GetDisplayName "/Game/ThirdPersonCPP/Blueprints/eyeCharCharacter.eyeCharCharacter"))
    (bind _output_get (Variables|Default|Setnum (+ (Variables|Default|Getnum) 1)))
    (if (>= _output_get 2)
      (Actor|DestroyActor)
      (Game|Damage|ApplyDamage (.AsEye%20Char%20Character (Utilities|Casting|CastToeyeCharCharacter (Game|GetPlayerCharacter 0))) 1.0 0 0))))

(fn ConstructionScript)